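; BP_Button is an actor that acts as a VR button, reacting visually when a BP_MotionController overlaps it.
; Begin and end overlap events cast to the controller and set or clear an Overlapping flag.
; Every Tick snaps the whole actor to TransformOverlap or TransformNoOverlap based on that flag, with no interpolation.
; The button triggers no other action.
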(event EventBeginPlay)

(event Collision|EventActorBeginOverlap
  (params (OtherActor :type Actor%20Object%20Reference))
  (Utilities|Casting|CastToBP_MotionController OtherActor)
  (Variables|Default|SetOverlapping true))

(event EventTick
  (params (DeltaSeconds :type Float%20%28single-precision%29))
  (if (Variables|Default|GetOverlapping)
    (Transformation|SetActorTransform (Variables|Default|GetTransformOverlap))
    (else
      (Transformation|SetActorTransform (Variables|Default|GetTransformNoOverlap)))))

(event Collision|EventActorEndOverlap
  (params (OtherActor :type Actor%20Object%20Reference))
  (Utilities|Casting|CastToBP_MotionController OtherActor)
  (Variables|Default|SetOverlapping false))

(fn ConstructionScript)